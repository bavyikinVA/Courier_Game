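; BP_WB_Enemy is a sprite-based enemy character that patrols along the X axis and deals contact damage.
; Despite its name, Follow runs each Tick as a patrol, counting S1 toward signed limit S, then negating S and flipping the sprite.
; BoxHit overlaps damage the other actor, pass the enemy's X to the cached player, and knock the enemy away from the player, briefly locking movement.
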(event `self.ReceiveBeginPlay`
  (bind _asbp_players (cast `/Game/Blueprints/Characters/Players/BP_Players` (`GameplayStatics.GetPlayerCharacter` 0)))
  (set `self.BP Players` _asbp_players))

(event `self.BoxHit.OnComponentBeginOverlap`
  (params (OverlappedComponent :type "PrimitiveComponent Object Reference") (OtherActor :type "Actor Object Reference") (OtherComp :type "PrimitiveComponent Object Reference") (OtherBodyIndex :type Integer) (bFromSweep :type Boolean) (SweepResult :type "HitResult Structure (by ref)"))
  (bind _returnvalue_x (`KismetMathLibrary.BreakVector` (`SceneComponent.K2_GetComponentLocation` (`self.Sprite`))))
  (bind _returnvalue_x_2 (`KismetMathLibrary.BreakVector` (`SceneComponent.K2_GetComponentLocation` (`self.Sprite`))))
  (bind _returnvalue_x_3 (`KismetMathLibrary.BreakVector` (`SceneComponent.K2_GetComponentLocation` (`PaperCharacter.Sprite` (`self.BP Players`)))))
  (set `/Game/Blueprints/Characters/Players/BP_Players.EnemyPositionnX` _returnvalue_x (`self.BP Players`))
  (`GameplayStatics.ApplyDamage` OtherActor 10.0)
  (`/Engine/EditorBlueprintResources/StandardMacros.CompareFloat` _returnvalue_x_3 _returnvalue_x_2
    (:`>`
      (`self.LaunchCharacter` (-500.0 0.0 0.0) true))
    (:`<`
      (`self.LaunchCharacter` (500.0 0.0 0.0) true)))
  (set `self.is Movement lock` true)
  (`KismetSystemLibrary.Delay` 1.0)
  (set `self.is Movement lock` false))

(event `self.ReceiveTick`
  (params (DeltaSeconds :type "Float (single-precision)"))
  (`self.Follow`))

(event `Follow`
  ;[1 1 1] Move Enemy
  (if (not (`self.is Movement lock`))
    (`/Engine/EditorBlueprintResources/StandardMacros.CompareFloat` (`self.S1`) (`self.S`)
      (:`>`
        (`self.AddMovementInput` (-1.0 0.0 0.0))
        (set `self.S1` (- (`self.S1`) 1.0)))
      (:`==`
        (if (> (`self.S`) 0.0)
          (set `self.S` (* (`self.S`) -1.0))
          (set `self.S1` 0.0)
          (`SceneComponent.K2_SetRelativeRotation` (`self.Sprite`) (struct :`Yaw` 180.0) false false)
          (else
            (set `self.S` (* (`self.S`) -1.0))
            (set `self.S1` 0.0)
            (`SceneComponent.K2_SetRelativeRotation` (`self.Sprite`) (struct) false false))))
      (:`<`
        (`self.AddMovementInput` (1.0 0.0 0.0))
        (set `self.S1` (+ (`self.S1`) 1.0))))))

(fn `UserConstructionScript`)